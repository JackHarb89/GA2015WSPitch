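; Pitch_Screen is an actor Blueprint that controls playback on an object named UE4, apparently the media for a pitch screen.
; Each ButtonActivated event switches on a ButtonPressed counter to cycle through Play, Pause and Rewind.
; Play and Pause advance the counter, and Rewind resets it to zero without calling Play.
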(event `self.ReceiveBeginPlay`)

(event `self.ReceiveActorBeginOverlap`
  (params (OtherActor :type "Actor Object Reference")))

(event `self.ReceiveTick`
  (params (DeltaSeconds :type "Float (single-precision)")))

(event `ButtonActivated`
  (switch `int` (`self.ButtonPressed`)
    (:`0`
      (`MediaPlayer.Play` (`self.UE4`))
      (bind _result (`/Engine/EditorBlueprintResources/StandardMacros.IncrementInt` (`self.ButtonPressed`) :!label _label)
        (:`  `
          (set `self.ButtonPressed` _result))))
    (:`1`
      (`MediaPlayer.Pause` (`self.UE4`))
      (goto _label))
    (:`2`
      (`MediaPlayer.Rewind` (`self.UE4`))
      (set `self.ButtonPressed` 0))))

(fn `UserConstructionScript`)